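; Turret enemy spawner that periodically creates BP_Enemy_Turret actors along a line between two arrow components.
; On BeginPlay it resets a random stream and sets a timer with a random delay.
; Each spawn takes the left arrow's X, Z and rotation with a random Y between both arrows, then re-queues the timer to repeat indefinitely.
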(event Custom|QueueTimer
  (Utilities|Time|SetTimerbyEvent (delegate Custom|SpawnEnemy) (Math|Random|RandomFloatinRangefromStream (Variables|Default|GetStream) 5.0 12.0)))

(event Custom|SpawnEnemy
  (bind _arrowleftside (Variables|Default|GetArrowLeftSide))
  (bind _returnvalue (Transformation|GetWorldLocation _arrowleftside))
  (Game|SpawnActorfromClass "/Game/Blueprints/BP_Enemy_Turret.BP_Enemy_Turret_C" (Math|Transform|MakeTransform (Math|Vector|MakeVector (.x _returnvalue) (Math|Random|RandomFloatinRangefromStream (Variables|Default|GetStream) (.y _returnvalue) (.y (Transformation|GetWorldLocation (Variables|Default|GetArrowRightSide)))) (.z _returnvalue)) (Transformation|GetWorldRotation _arrowleftside) "1.000000,1.000000,1.000000") "Undefined" "MultiplyWithRoot" 0 0)
  (CallFunction|QueueTimer))

(event EventBeginPlay
  (Class|KismetMathLibrary|ResetRandomStream (Variables|Default|GetStream))
  (CallFunction|QueueTimer))

(fn ConstructionScript)