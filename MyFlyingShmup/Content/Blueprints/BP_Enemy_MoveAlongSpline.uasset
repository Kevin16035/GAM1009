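; Enemy actor that travels along a path shaped by its Spline, starting on BeginPlay.
; A slowed Timeline samples the spline's local location at constant velocity and sweeps the actor to its initial transform relative to that point, so the offset is subtracted, mirroring the path.
; The Mesh turns from the spline's right vector plus a 180-degree offset, sampled without constant velocity, unlike the position.
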(event EventBeginPlay
  (|CallParentFunction)
  (Components|Timeline|SetPlayRate (Variables|Default|GetTimeline) 0.1)
  (Variables|Default|SetInitialTransform (Transformation|GetActorTransform))
  (bind _progress (Timeline|Timeline PlayFromStart)
    (:Update
      (bind _spline (Variables|Default|GetSpline)
        (:then
          (Transformation|SetActorTransform (Math|Transform|MakeRelativeTransform (Variables|Default|GetInitialTransform) (Math|Transform|MakeTransform (Spline|GetLocationatTime _spline _progress "Local" true))) true)
          (Transformation|SetRelativeRotation (Variables|Character|GetMesh) (Math|Rotator|CombineRotators (Math|Rotator|MakeRotfromY (Class|SplineComponent|GetRightVectoratTime _spline _progress "Local" false)) "0.000000,180.000000,0.000000") false false))
        (:else)))))

(event Collision|EventActorBeginOverlap
  (params (OtherActor :type Actor%20Object%20Reference))
  (|CallParentFunction OtherActor) ; This node is disabled and will not be called.\nDrag off pins to build functionality.
)

(event EventTick
  (params (DeltaSeconds :type Float%20%28single-precision%29)))

(fn ConstructionScript
  (|CallParentFunction))