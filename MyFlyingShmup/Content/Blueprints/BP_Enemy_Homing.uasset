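; BP_Enemy_Homing is an enemy Blueprint that uses a projectile movement component to home in on the first player's pawn.
; BeginPlay calls the parent, then sets the pawn's root component as the homing target, and Tick repeats that assignment every frame.
; An older yaw-based approach that sets velocity toward the player is left unconnected, and the overlap event is disabled.
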(event EventBeginPlay
  (|CallParentFunction)
  (Variables|/Script/Engine.ProjectileMovementComponent|SetHomingTargetComponent (Variables|Default|GetProjectileMovement) (Variables|/Script/Engine.Actor|GetRootComponent (Game|Player|GetPlayerPawn 0))))

(event Collision|EventActorBeginOverlap
  (params (OtherActor :type Actor%20Object%20Reference))
  (|CallParentFunction OtherActor) ; This node is disabled and will not be called.\nDrag off pins to build functionality.
)

(event EventTick
  (params (DeltaSeconds :type Float%20%28single-precision%29))
  (Variables|/Script/Engine.ProjectileMovementComponent|SetHomingTargetComponent (Variables|Default|GetProjectileMovement) (Variables|/Script/Engine.Actor|GetRootComponent (Game|Player|GetPlayerPawn 0))))

(fn ConstructionScript
  (|CallParentFunction))