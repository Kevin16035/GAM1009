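; BP_Enemy_Turret is a stationary enemy that periodically turns toward the player and fires a 2D bullet.
; A looping two-second timer started on BeginPlay restarts a FireSequence timeline.
; While it plays, the turret smoothly interpolates only its yaw toward the player pawn.
; When the timeline finishes, it spawns BP_Bullet2D_Enemy at the FireSpawnPoint component's location and rotation.
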(event Custom|StartShooting
  (Utilities|Time|SetTimerbyEvent (delegate Custom|FacePlayer) 2.0 true))

(event Custom|FacePlayer
  (Timeline|FireSequence PlayFromStart
    (:Update
      (bind _output_get (Variables|Default|SetTargetYaw (.yaw (Math|Rotator|FindLookatRotation (Transformation|GetActorLocation) (Transformation|GetActorLocation (Game|Player|GetPlayerPawn 0))))))
      (bind _output_get_2 (Variables|Default|SetCurrentYaw (.yaw (Math|Interpolation|RInterpTo (Math|Rotator|MakeRotator 0.0 0.0 (Variables|Default|GetCurrentYaw)) (Math|Rotator|MakeRotator 0.0 0.0 _output_get) (Utilities|Time|GetWorldDeltaSeconds) 2.0))))
      (Transformation|SetActorRotation (Math|Rotator|MakeRotator 0.0 0.0 _output_get_2)))
    (:Finished
      (CallFunction|FireBullet))))

(event Custom|FireBullet
  (bind _firespawnpoint (Variables|Default|GetFireSpawnPoint))
  (Game|SpawnActorfromClass "/Game/Blueprints/BP_Bullet2D_Enemy.BP_Bullet2D_Enemy_C" (Math|Transform|MakeTransform (Transformation|GetWorldLocation _firespawnpoint) (Transformation|GetWorldRotation _firespawnpoint) "1.000000,1.000000,1.000000") "Undefined" "MultiplyWithRoot" 0 0))

(event EventBeginPlay
  (|CallParentFunction)
  (CallFunction|StartShooting))

(fn ConstructionScript
  (|CallParentFunction))