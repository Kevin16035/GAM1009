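; Boss enemy Blueprint that enters along a spline, then moves along Y while firing volleys of enemy bullets.
; A half-speed timeline drives constant-velocity spline movement relative to the spawn transform, then hands off to the LeftToRight timeline for swept lateral movement.
; From BeginPlay, a looping timer runs in parallel, spawning BP_Bullet2D_Enemy at each of six arrow components' world location and rotation.
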(event Custom|BeginRegularShooting
  (Utilities|Time|SetTimerbyEvent (delegate Custom|SpawnBullet) 1.5 true))

(event Custom|SpawnBullet
  (for _array_element (Utilities|Array|MakeArray (Variables|Default|GetArrow4) (Variables|Default|GetArrow3) (Variables|Default|GetArrow2) (Variables|Default|GetArrow1) (Variables|Default|GetArrow5) (Variables|Default|GetArrow))
    (Game|SpawnActorfromClass "/Game/Blueprints/BP_Bullet2D_Enemy.BP_Bullet2D_Enemy_C" (Math|Transform|MakeTransform (.location (Transformation|GetWorldTransform _array_element)) (.rotation (Transformation|GetWorldTransform _array_element)) "1.000000,1.000000,1.000000") "Undefined" "MultiplyWithRoot" 0 0)))

(event EventBeginPlay
  (|CallParentFunction)
  (Components|Timeline|SetPlayRate (Variables|Default|GetTimeline) 0.5)
  (Variables|Default|SetInitialTransform (Transformation|GetActorTransform))
  (Utilities|FlowControl|Sequence
    (:then_0
      (bind _progress (Timeline|Timeline PlayFromStart)
        (:Update
          (bind _spline (Variables|Default|GetSpline)
            (:then
              (Transformation|SetActorTransform (Math|Transform|MakeRelativeTransform (Variables|Default|GetInitialTransform) (Math|Transform|MakeTransform (Spline|GetLocationatTime _spline _progress "Local" true))) true))
            (:else)))
        (:Finished
          (Variables|Default|SetInitialTransform "")
          (bind _value (Timeline|LeftToRight PlayFromStart)
            (:Update
              (Transformation|SetActorTransform (Math|Transform|MakeRelativeTransform (Math|Transform|MakeTransform (Math|Vector|MakeVector 0.0 (* _value 1.5e+03) 0.0) "0, 0, 0" "1.000000,1.000000,1.000000") (Variables|Default|GetInitialTransform)) true))))))
    (:then_1
      (CallFunction|BeginRegularShooting))))

(fn ConstructionScript
  (|CallParentFunction))