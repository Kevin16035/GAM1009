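; Player pawn for a shooter, moved through Enhanced Input and FloatingPawnMovement.
; Delayed primary fire uses one of three modes, switched by debug keys: single shot, alternating muzzles, or a centered fan spray.
; Damage lowers clamped health with camera shake and red overlay flash, while overlapping actors receive damage equal to the pawn's health.
; At zero health it spawns and possesses a replacement at a PlayerStart, then destroys itself with an explosion effect.
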(event Custom|ApplyCameraShake
  (Camera|PlayWorldCameraShake "/Game/Blueprints/BP_CameraShake.BP_CameraShake_C" "0, 0, 0" 0.0 1e+04))

(event Custom|CheckHealth
  (if (== (Variables|Default|GetHealth) 0.0)
    (CallFunction|OnDeath)))

(event Custom|OnDeath
  (bind _returnvalue (Actor|GetActorOfClass "/Script/Engine.PlayerStart"))
  (Utilities|IsValid 0
    (:Is%20Valid
      (bind _returnvalue_2 (Game|SpawnActorfromClass "BP_PlayerPawn_C" (Transformation|GetActorTransform _returnvalue) "Undefined" "MultiplyWithRoot" 0 0))
      (bind _asplayer_controller (Utilities|Casting|CastToPlayerController (Pawn|GetController)))
      (Pawn|Possess _asplayer_controller _returnvalue_2)
      (Actor|DestroyActor)
      (Niagara|SpawnSystematLocation "/Game/Particles/FX_EnemyExplosion_System.FX_EnemyExplosion_System" (Transformation|GetActorLocation)))))

(event Custom|FlashRedOverlayMaterial
  (Rendering|Material|SetOverlayMaterial (Variables|Default|GetMesh) "/Game/Materials/M_OverlayWhenHit.M_OverlayWhenHit" :!class /Script/Engine.MeshComponent)
  (Utilities|FlowControl|Delay 0.2)
  (Rendering|Material|SetOverlayMaterial (Variables|Default|GetMesh) 0 :!class /Script/Engine.MeshComponent))

(event Input|EnhancedActionEvents|EnhancedInputActionIA_MoveForwardBackward
  (params (ActionValue :type Float%20%28double-precision%29) (ElapsedSeconds :type Float%20%28double-precision%29) (TriggeredSeconds :type Float%20%28double-precision%29) (InputAction :type Input%20Action%20Object%20Reference :default "/Game/Inputs/IA_MoveForwardBackward.IA_MoveForwardBackward"))
  (Class|PawnMovementComponent|AddInputVector (Variables|Default|GetFloatingPawnMovement) (Math|Vector|MakeVector ActionValue 0.0 0.0) false))

(event Input|EnhancedActionEvents|EnhancedInputActionIA_MoveRightLeft
  (params (ActionValue :type Float%20%28double-precision%29) (ElapsedSeconds :type Float%20%28double-precision%29) (TriggeredSeconds :type Float%20%28double-precision%29) (InputAction :type Input%20Action%20Object%20Reference :default "/Game/Inputs/IA_MoveRightLeft.IA_MoveRightLeft"))
  (Class|PawnMovementComponent|AddInputVector (Variables|Default|GetFloatingPawnMovement) (Math|Vector|MakeVector 0.0 ActionValue 0.0) false))

(event Input|EnhancedActionEvents|EnhancedInputActionIA_PrimaryFire
  (params (ActionValue :type Boolean) (ElapsedSeconds :type Float%20%28double-precision%29) (TriggeredSeconds :type Float%20%28double-precision%29) (InputAction :type Input%20Action%20Object%20Reference :default "/Game/Inputs/IA_PrimaryFire.IA_PrimaryFire"))
  (bind _primaryfirespawnpoint1 (Variables|Default|GetPrimaryFireSpawnPoint1))
  (bind _primaryfirespawnpoint1_2 (Variables|Default|GetPrimaryFireSpawnPoint1))
  (bind _numberofbulletstospray (Variables|Default|GetNumberOfBulletsToSpray))
  (bind _angleofspraybullets (Variables|Default|GetAngleOfSprayBullets))
  (bind _returnvalue (Transformation|GetWorldTransform _primaryfirespawnpoint1_2))
  (bind _returnvalue_2 (Math|Vector|GetForwardVector _primaryfirespawnpoint1))
  (bind _returnvalue_3 (Math|Rotator|MakeRotfromX _returnvalue_2))
  (Utilities|FlowControl|Delay 0.2)
  (switch int (Variables|Default|GetShootingModeIndex)
    (:0
      ;[0.15 0.15 0.15 0.5] Shooting Mode 1
      (Game|SpawnActorfromClass "/Game/Blueprints/BP_Bullet2D_Player.BP_Bullet2D_Player_C" (Math|Transform|MakeTransform (.location _returnvalue) (.rotation _returnvalue) "1.000000,1.000000,1.000000") "Undefined" "MultiplyWithRoot" 0 0))
    (:1
      ;[0.15 0.15 0.15 0.5] Shooting Mode 2
      (bind _isa (Utilities|FlowControl|FlipFlop)
        (:A
          _)
        (:B
          _))
      (Game|SpawnActorfromClass "/Game/Blueprints/BP_Bullet2D_Player.BP_Bullet2D_Player_C" (Math|Transform|MakeTransform (.location (Transformation|GetWorldTransform (select _isa (Variables|Default|GetPrimaryFireSpawnPoint2) (Variables|Default|GetPrimaryFireSpawnPoint3)))) (.rotation (Transformation|GetWorldTransform (select _isa (Variables|Default|GetPrimaryFireSpawnPoint2) (Variables|Default|GetPrimaryFireSpawnPoint3)))) "1.000000,1.000000,1.000000") "Undefined" "MultiplyWithRoot" 0 0))
    (:2
      ;[0.15 0.15 0.15 0.5] Shooting Mode 3
      (for _index (range 1 (Variables|Default|GetNumberOfBulletsToSpray))
        (Game|SpawnActorfromClass "/Game/Blueprints/BP_Bullet2D_Player.BP_Bullet2D_Player_C" (Math|Transform|MakeTransform (Transformation|GetWorldLocation _primaryfirespawnpoint1) (Math|Rotator|MakeRotator (.roll _returnvalue_3) (.pitch _returnvalue_3) (+ (.yaw _returnvalue_3) (Utilities|Operators|Subtract (* _index _angleofspraybullets) (* (Math|Float|Round (* _numberofbulletstospray 0.5)) (Variables|Default|GetAngleOfSprayBullets)) (Utilities|Select :Index (Math|Integer|%(Integer) _numberofbulletstospray 2) :Option%200 (* _angleofspraybullets 0.5) :Option%201 0.0)))) "1.000000,1.000000,1.000000") "Undefined" "MultiplyWithRoot" 0 0)))))

(event Collision|EventActorBeginOverlap
  (params (OtherActor :type Actor%20Object%20Reference))
  (Game|Damage|ApplyDamage OtherActor (Variables|Default|GetHealth) 0 0))

(event Game|Damage|EventAnyDamage
  (params (Damage :type Float%20%28single-precision%29) (DamageType :type Damage%20Type%20Object%20Reference) (InstigatedBy :type Controller%20Object%20Reference) (DamageCauser :type Actor%20Object%20Reference))
  (Variables|Default|SetHealth (Math|Float|Clamp(Float) (- (Variables|Default|GetHealth) Damage) 0.0 (Variables|Default|GetMaxHealth)))
  (CallFunction|ApplyCameraShake)
  (CallFunction|FlashRedOverlayMaterial)
  (CallFunction|CheckHealth))

(event EventBeginPlay
  (Collision|SetCollisionEnabled (Variables|Default|GetSphere) "NoCollision")
  (Utilities|FlowControl|Delay 2.0)
  (Class|PrimitiveComponent|SetNotifyRigidBodyCollision (Variables|Default|GetSphere) false))

(event EventPossessed
  (params (NewController :type Controller%20Object%20Reference))
  (bind _asplayer_controller (Utilities|Casting|CastToPlayerController NewController))
  (Input|AddMappingContext (PlayerController|LocalPlayerSubsystems|GetEnhancedInputLocalPlayerSubsystem _asplayer_controller) "/Game/Inputs/IMC_PlayerInputs.IMC_PlayerInputs" 0 "(bIgnoreAllPressedKeysUntilRelease=True,bForceImmediately=False,bNotifyUserSettings=False)"))

(event Input|KeyboardEvents|DebugKeyN
  (params (Key :type Key%20Structure :default "None") (ActionValue :type Input%20Action%20Value%20Structure))
  ;[0.15 0.15 0.15 0.5] change shooting modes
  (:Pressed
    (Variables|Default|SetShootingModeIndex (Math|Integer|Clamp(Integer) (+ (Variables|Default|GetShootingModeIndex) 1) 0 2))))

(event Input|KeyboardEvents|DebugKeyM
  (params (Key :type Key%20Structure :default "None") (ActionValue :type Input%20Action%20Value%20Structure))
  ;[0.15 0.15 0.15 0.5] change shooting modes
  (:Pressed
    (Variables|Default|SetShootingModeIndex (Math|Integer|Clamp(Integer) (- (Variables|Default|GetShootingModeIndex) 1) 0 2))))

(fn ConstructionScript)