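; Wave manager that spawns timed enemy waves from a data asset.
; Chained events step through waves and their enemy groups, spawning each enemy after a short random delay from a seeded stream.
; Regular enemies spawn at random Y between LeftMax and RightMax, while boss waves use a fixed point and switch the music through the GameInstance.
; Spawns receive optional pickup drops, and final-wave boss spawns are flagged as the level's last enemy.
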(event Custom|SpawnNextWave
  (bind _waves (Variables|Default|GetWaves))
  (bind _currentwaveindex (Variables|Default|GetCurrentWaveIndex))
  (bind _leftmax (Variables|Default|GetLeftMax))
  (bind _returnvalue (Transformation|GetWorldLocation _leftmax))
  (bind _output (Utilities|Array|Get(acopy) _waves _currentwaveindex))
  (bind _result (Math|Integer|IncrementInt _currentwaveindex)
    (:%20%20
      (if (Utilities|Array|IsValidIndex _waves)
        (Utilities|FlowControl|Delay (.initialdelay _output))
        (Development|PrintString (Utilities|String|Append "spawning wave" (Utilities|String|ToString(Integer) _result)))
        (if (.isbosswave _output)
          (Class|BPIMyFlyingShmup|PlayMusic(Message) (Game|GetGameInstance) "/Game/AbsoluteSpaceAndSciFi_VoltzSupreme/Cues/Hyper_-_No_Noise__High_or_Build_Cue.Hyper_-_No_Noise__High_or_Build_Cue" false))
        (Variables|Default|SetCurrentEnemiesData (.enemies _output))
        (bind _output_get (Variables|Default|SetCurrentEnemiesIndex -1))
        (bind _result_2 (Math|Integer|IncrementInt _output_get)
          (:%20%20
            (Development|PrintString (Utilities|String|Append "current enemy index" (Utilities|String|ToString(Integer) _result_2)))
            (if (Utilities|Array|IsValidIndex (Variables|Default|GetCurrentEnemiesData) _result_2)
              (Variables|Default|SetMaxEnemyCount (.enemycount (Utilities|Array|Get(acopy) (Variables|Default|GetCurrentEnemiesData) (Variables|Default|GetCurrentEnemiesIndex))))
              (bind _output_get_2 (Variables|Default|SetCurrentEnemyCount 0))
              (if (< _output_get_2 (Variables|Default|GetMaxEnemyCount)) :!label _label
                (Game|SpawnActorfromClass (.enemyclass (Utilities|Array|Get(acopy) (Variables|Default|GetCurrentEnemiesData) (Variables|Default|GetCurrentEnemiesIndex))) (Math|Transform|MakeTransform (select (.isbosswave _output) "2000.000000,0.000000,0.000000" (Math|Vector|MakeVector (.x _returnvalue) (Math|Random|RandomFloatinRangefromStream (Variables|Default|GetStream) (.y _returnvalue) (.y (Transformation|GetWorldLocation (Variables|Default|GetRightMax)))) (.z _returnvalue))) (Transformation|GetWorldRotation _leftmax) "1.000000,1.000000,1.000000") "AlwaysSpawn" "MultiplyWithRoot" 0 (select (.candroppickup (Utilities|Array|Get(acopy) (Variables|Default|GetCurrentEnemiesData) (Variables|Default|GetCurrentEnemiesIndex))) (.pickupclass (Utilities|Array|Get(acopy) (Variables|Default|GetCurrentEnemiesData) (Variables|Default|GetCurrentEnemiesIndex))) 0) (and (.isbosswave _output) (== (Variables|Default|GetCurrentWaveIndex) (- (Variables|Default|GetNumberOfWaves) 1))) 0)
                (Math|Integer|IncrementInt (Variables|Default|GetCurrentEnemyCount)
                  (:%20%20
                    (Utilities|FlowControl|Delay (Math|Random|RandomFloatinRangefromStream (Variables|Default|GetStream) 1.0 2.0))
                    (goto _label)))
                (else
                  (CallFunction|SpawnNextEnemiesinCurrentWave)))
              (else
                (CallFunction|SpawnNextWave)))))
        (else
          (Development|PrintString "No more waves in data assett to spawn"))))))

(event Custom|StartSpawningWaves
  (bind _waves (Variables|Default|GetWaves))
  (bind _currentwaveindex (Variables|Default|GetCurrentWaveIndex))
  (bind _leftmax (Variables|Default|GetLeftMax))
  (bind _returnvalue (Transformation|GetWorldLocation _leftmax))
  (bind _output (Utilities|Array|Get(acopy) _waves _currentwaveindex))
  (Utilities|FlowControl|Delay (.initialdelay _output))
  (Development|PrintString (Utilities|String|Append "spawning wave" (Utilities|String|ToString(Integer) (stale Custom|SpawnNextWave _result))))
  (if (.isbosswave _output)
    (Class|BPIMyFlyingShmup|PlayMusic(Message) (Game|GetGameInstance) "/Game/AbsoluteSpaceAndSciFi_VoltzSupreme/Cues/Hyper_-_No_Noise__High_or_Build_Cue.Hyper_-_No_Noise__High_or_Build_Cue" false))
  (Variables|Default|SetCurrentEnemiesData (.enemies _output))
  (bind _output_get (Variables|Default|SetCurrentEnemiesIndex -1))
  (bind _result (Math|Integer|IncrementInt _output_get)
    (:%20%20
      (Development|PrintString (Utilities|String|Append "current enemy index" (Utilities|String|ToString(Integer) _result)))
      (if (Utilities|Array|IsValidIndex (Variables|Default|GetCurrentEnemiesData) _result)
        (Variables|Default|SetMaxEnemyCount (.enemycount (Utilities|Array|Get(acopy) (Variables|Default|GetCurrentEnemiesData) (Variables|Default|GetCurrentEnemiesIndex))))
        (bind _output_get_2 (Variables|Default|SetCurrentEnemyCount 0))
        (if (< _output_get_2 (Variables|Default|GetMaxEnemyCount)) :!label _label
          (Game|SpawnActorfromClass (.enemyclass (Utilities|Array|Get(acopy) (Variables|Default|GetCurrentEnemiesData) (Variables|Default|GetCurrentEnemiesIndex))) (Math|Transform|MakeTransform (select (.isbosswave _output) "2000.000000,0.000000,0.000000" (Math|Vector|MakeVector (.x _returnvalue) (Math|Random|RandomFloatinRangefromStream (Variables|Default|GetStream) (.y _returnvalue) (.y (Transformation|GetWorldLocation (Variables|Default|GetRightMax)))) (.z _returnvalue))) (Transformation|GetWorldRotation _leftmax) "1.000000,1.000000,1.000000") "AlwaysSpawn" "MultiplyWithRoot" 0 (select (.candroppickup (Utilities|Array|Get(acopy) (Variables|Default|GetCurrentEnemiesData) (Variables|Default|GetCurrentEnemiesIndex))) (.pickupclass (Utilities|Array|Get(acopy) (Variables|Default|GetCurrentEnemiesData) (Variables|Default|GetCurrentEnemiesIndex))) 0) (and (.isbosswave _output) (== (Variables|Default|GetCurrentWaveIndex) (- (Variables|Default|GetNumberOfWaves) 1))) 0)
          (Math|Integer|IncrementInt (Variables|Default|GetCurrentEnemyCount)
            (:%20%20
              (Utilities|FlowControl|Delay (Math|Random|RandomFloatinRangefromStream (Variables|Default|GetStream) 1.0 2.0))
              (goto _label)))
          (else
            (CallFunction|SpawnNextEnemiesinCurrentWave)))
        (else
          (CallFunction|SpawnNextWave))))))

(event Custom|SpawnNextEnemiesInCurrentWave
  (bind _waves (Variables|Default|GetWaves))
  (bind _currentwaveindex (Variables|Default|GetCurrentWaveIndex))
  (bind _currentenemiesindex (Variables|Default|GetCurrentEnemiesIndex))
  (bind _currentenemiesdata (Variables|Default|GetCurrentEnemiesData))
  (bind _leftmax (Variables|Default|GetLeftMax))
  (bind _returnvalue (Transformation|GetWorldLocation _leftmax))
  (bind _output (Utilities|Array|Get(acopy) _waves _currentwaveindex))
  (bind _output_2 (Utilities|Array|Get(acopy) _currentenemiesdata _currentenemiesindex))
  (bind _result (Math|Integer|IncrementInt (stale Custom|SpawnNextWave _output_get))
    (:%20%20
      (Development|PrintString (Utilities|String|Append "current enemy index" (Utilities|String|ToString(Integer) _result)))
      (if (Utilities|Array|IsValidIndex _currentenemiesdata _result)
        (Variables|Default|SetMaxEnemyCount (.enemycount _output_2))
        (bind _output_get (Variables|Default|SetCurrentEnemyCount 0))
        (if (< _output_get (Variables|Default|GetMaxEnemyCount)) :!label _label
          (Game|SpawnActorfromClass (.enemyclass _output_2) (Math|Transform|MakeTransform (select (.isbosswave _output) "2000.000000,0.000000,0.000000" (Math|Vector|MakeVector (.x _returnvalue) (Math|Random|RandomFloatinRangefromStream (Variables|Default|GetStream) (.y _returnvalue) (.y (Transformation|GetWorldLocation (Variables|Default|GetRightMax)))) (.z _returnvalue))) (Transformation|GetWorldRotation _leftmax) "1.000000,1.000000,1.000000") "AlwaysSpawn" "MultiplyWithRoot" 0 (select (.candroppickup _output_2) (.pickupclass _output_2) 0) (and (.isbosswave _output) (== (Variables|Default|GetCurrentWaveIndex) (- (Variables|Default|GetNumberOfWaves) 1))) 0)
          (Math|Integer|IncrementInt (Variables|Default|GetCurrentEnemyCount)
            (:%20%20
              (Utilities|FlowControl|Delay (Math|Random|RandomFloatinRangefromStream (Variables|Default|GetStream) 1.0 2.0))
              (goto _label)))
          (else
            (CallFunction|SpawnNextEnemiesinCurrentWave)))
        (else
          (CallFunction|SpawnNextWave))))))

(event EventBeginPlay
  (Class|KismetMathLibrary|ResetRandomStream (Variables|Default|GetStream))
  (Variables|Default|SetWaves (Variables|/Game/Blueprints/PDA_SetOfWaves.PDA_SetOfWaves_C|GetWaves (Variables|Default|GetWavesDataAsset)))
  (Variables|Default|SetNumberOfWaves (Utilities|Array|Length (Variables|/Game/Blueprints/PDA_SetOfWaves.PDA_SetOfWaves_C|GetWaves (Variables|Default|GetWavesDataAsset))))
  (CallFunction|StartSpawningWaves))

(fn ConstructionScript)